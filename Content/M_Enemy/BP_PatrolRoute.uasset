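; BP_PatrolRoute is a patrol path actor that supplies spline points as waypoints, apparently for enemy movement.
; IncrementPatrolRoute steps PatrolIndex by Direction, reversing it at the last and first spline points so the route ping-pongs end to end.
; GetSplinePointAsWorldPosition returns the world location of the PatrolRoute spline point at the current index.
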(event `IncrementPatrolRoute`
  (bind _output_get (set `self.PatrolIndex` (+ (`self.PatrolIndex`) (`self.Direction`)))) ; 设置最新节点
  (if (== _output_get (- (`SplineComponent.GetNumberOfSplinePoints` (`self.PatrolRoute`)) 1))
    (set `self.Direction` -1) ; 将方向重置为负方向
    (elif (== (`self.PatrolIndex`) 0)
      (set `self.Direction` 1) ; 走完前方向将一直为这个方向
    )))

(fn `GetSplinePointAsWorldPosition`
  (returns (Location :type "Vector Structure"))
  (return (`SplineComponent.GetLocationAtSplinePoint` (`self.PatrolRoute`) (`self.PatrolIndex`) "World")))

(fn `UserConstructionScript`)