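; Ranged enemy character that carries a gun in each hand and performs a montage-driven attack.
; On BeginPlay, two custom events each spawn a BP_Gun and snap it to the right or left hand socket on the mesh.
; Attack prints a temporary debug message and plays the ranged attack montage slightly sped up, calling OnAttackEnd whether it completes or is interrupted.
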(event `self.ReceiveBeginPlay`
  (`self.Gun`)
  (`self.GUn2`))

(event `/Game/M_Enemy/BPI_EnemyAI.Attack`
  (`KismetSystemLibrary.PrintString` "播放攻击蒙太奇！") ; debug一下，后面记得自己删了
  (`|PlayMontage` (`self.Mesh`) "/Game/M_Enemy/EnemyAnime/RangedAttack_Enemy.RangedAttack_Enemy" 1.3 ; 播放攻击蒙太奇
    (:`OnCompleted`
      _)
    (:`OnInterrupted`
      _))
  (`self.OnAttackEnd`) ; 调用事件
)

(event `Gun`
  (bind _returnvalue (`|SpawnActorFromClass` "/Game/M_Enemy/Weapon/BP_Gun.BP_Gun_C" (`self.GetTransform`) "Undefined" "MultiplyWithRoot" null null))
  (`self.K2_AttachToComponent` _returnvalue (`self.Mesh`) "hand_rSocket" "SnapToTarget" "SnapToTarget" "SnapToTarget" true))

(event `GUn2`
  (bind _returnvalue (`|SpawnActorFromClass` "/Game/M_Enemy/Weapon/BP_Gun.BP_Gun_C" (`self.GetTransform`) "Undefined" "MultiplyWithRoot" null null))
  (`self.K2_AttachToComponent` _returnvalue (`self.Mesh`) "hand_lSocket" "SnapToTarget" "SnapToTarget" "SnapToTarget" true))

(fn `UserConstructionScript`
  (`parent.UserConstructionScript`))